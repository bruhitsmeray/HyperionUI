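; HUI_Instance is a game instance Blueprint that loads the HUI save file and applies saved upscaling settings at startup.
; After a short delay, Init calls InitSaveGame, which loads the slot or creates and saves a new HUI_SaveFile, then re-runs itself to load it.
; Saved video settings then toggle FidelityFX FSR2 and, when enabled, set its quality and sharpness through formatted console commands.
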(event EventInit
  (bind _saveobject (Variables|Default|GetSaveObject))
  (bind _datavideosettings (Variables|/HyperionUI/Blueprints/HUI_SaveFile.HUI_SaveFile_C|GetDataVideoSettings _saveobject))
  (Utilities|FlowControl|Delay 0.2)
  (Utilities|FlowControl|Sequence
    (:then_0
      (CallFunction|InitSaveGame))
    (:then_1
      (switch int (.upscalingmethod (Variables|/HyperionUI/Blueprints/HUI_SaveFile.HUI_SaveFile_C|GetDataVideoSettings (Variables|Default|GetSaveObject)))
        (:0
          (CallFunction|EnableFSR))
        (:1
          (CallFunction|EnableFSR 1)
          (Utilities|FlowControl|Sequence
            (:then_0
              (CallFunction|SetFSRQuality (.upscalingquality _datavideosettings)))
            (:then_1
              (CallFunction|SetFSRSharpness (.upscalingsharpness _datavideosettings)))))))))

(fn InitSaveGame
  (bind _returnvalue (SaveGame|DoesSaveGameExist (Variables|Default|GetSaveName)))
  (if _returnvalue
    (bind _returnvalue_2 (SaveGame|LoadGamefromSlot (Variables|Default|GetSaveName)))
    (bind _ashui_save_file (Utilities|Casting|CastToHUI_SaveFile _returnvalue_2))
    (Variables|Default|SetSaveObject _ashui_save_file)
    (else
      (bind _returnvalue_3 (SaveGame|CreateSaveGameObject "/HyperionUI/Blueprints/HUI_SaveFile.HUI_SaveFile_C"))
      (bind _output_get (Variables|Default|SetSaveObject _returnvalue_3))
      (bind _returnvalue_4 (SaveGame|SaveGametoSlot _output_get (Variables|Default|GetSaveName)))
      (if _returnvalue_4
        (CallFunction|InitSaveGame)))))

(fn EnableFSR
  (params (Mode :type Integer))
  (Development|ExecuteConsoleCommand (Utilities|String|ToString(Text) (Utilities|Text|FormatText "r.FidelityFX.FSR2.Enabled {Mode}" Mode)) (Game|GetPlayerController 0)))

(fn SetFSRQuality
  (params (Mode :type Integer))
  (Development|ExecuteConsoleCommand (Utilities|String|ToString(Text) (Utilities|Text|FormatText "r.FidelityFX.FSR2.QualityMode {Mode}" Mode)) (Game|GetPlayerController 0)))

(fn SetFSRSharpness
  (params (Value :type Float%20%28single-precision%29))
  (Development|ExecuteConsoleCommand (Utilities|String|ToString(Text) (Utilities|Text|FormatText "r.FidelityFX.FSR2.Sharpness {Sharpness}" Value)) (Game|GetPlayerController 0)))